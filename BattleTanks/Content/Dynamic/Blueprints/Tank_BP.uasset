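; Player-controllable tank pawn that drives on tracks, fires and shows a health bar widget.
; BeginPlay hands barrel, turret and track parts to the TankAiming and TankMovement components, which handle firing and movement, and links the widget to this tank.
; Input handlers forward to those components, emit pawn noise and toggle first/third-person cameras.
; Firing sound plays only if rounds remain after the Fire call; gimbal rotation logic is disconnected.
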(event `self.ReceiveBeginPlay`
  (`TankAimingComponent.InitializeAim` (`self.TankAiming`) (`self.Barrel`) (`self.Turret`))
  (`TankMovementComponent.Initialize` (`self.TankMovement`) (`self.L_Track`) (`self.R_Track`))
  (`self.InitializeHealthBarWidget`))

(event `InputAction|Fire`
  (params (Key :type "Key Structure" :default "AnyKey"))
  ;[1 1 1] Fire input setup
  (:`Pressed`
    (`TankAimingComponent.Fire` (`self.TankAiming`))
    (`self.MakePawnNoise` 1.0)
    (`self.TankFireSound`)))

(event `InputAxis|MoveForward`
  (params (AxisValue :type "Float (single-precision)"))
  ;[1 1 1] Movement Input Binding
  (`TankMovementComponent.IntendMoveForward` (`self.TankMovement`) AxisValue)
  (`self.MakePawnNoise` 1.0 :!label _label))

(event `InputAxis|TurnRight`
  (params (AxisValue :type "Float (single-precision)"))
  ;[1 1 1] Movement Input Binding
  (`TankMovementComponent.IntendTurnRight` (`self.TankMovement`) AxisValue)
  (goto _label))

(event `InputAction|Swap Cam`
  (params (Key :type "Key Structure" :default "AnyKey"))
  ;[1 1 1] Camera Swapping
  (:`Pressed`
    (`ActorComponent.ToggleActive` (`self.3rd Person`))
    (`ActorComponent.ToggleActive` (`self.1st Person`))))

(fn `InitializeHealthBarWidget`
  (bind _ashealth_bar_bp (cast `/Game/Dynamic/Blueprints/HealthBar_BP` (`WidgetComponent.GetUserWidgetObject` (`self.Widget`)))
    (:`then`
      (set `/Game/Dynamic/Blueprints/HealthBar_BP.Tank` self _ashealth_bar_bp))
    (:`CastFailed`
      _))
  (return))

(fn `TankFireSound`
  (if (> (`TankAimingComponent.GetRoundsLeft` (`self.TankAiming`)) 0)
    (`self.MakeSoundTankFiring`)))

(fn `UserConstructionScript`)