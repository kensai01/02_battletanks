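; Terrain tile for the infinite terrain game mode, with a barrier and an attach point that exposes its world transform.
; The barrier starts solid, opens when anything enters LockingVolume, and closes on exit, which also asks the game mode to spawn a tile.
; The tile destroys itself when the player character enters DestroyVolume; the locking overlaps have no player check.
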(event `self.ReceiveBeginPlay`
  (`self.LockLevel`))

(event `self.LockingVolume.OnComponentBeginOverlap`
  (params (OverlappedComponent :type "PrimitiveComponent Object Reference") (OtherActor :type "Actor Object Reference") (OtherComp :type "PrimitiveComponent Object Reference") (OtherBodyIndex :type Integer) (bFromSweep :type Boolean) (SweepResult :type "HitResult Structure (by ref)"))
  (`self.UnlockLevel`))

(event `self.LockingVolume.OnComponentEndOverlap`
  (params (OverlappedComponent :type "PrimitiveComponent Object Reference") (OtherActor :type "Actor Object Reference") (OtherComp :type "PrimitiveComponent Object Reference") (OtherBodyIndex :type Integer))
  (`self.LockLevel`)
  (bind _asbattle_tank_game_mode_infinite_terrain_bp2 (cast `/Game/Dynamic/Blueprints/BattleTankGameMode_InfiniteTerrain_BP2` (`GameplayStatics.GetGameMode`)))
  (`/Game/Dynamic/Blueprints/BattleTankGameMode_InfiniteTerrain_BP2.SpawnTile` _asbattle_tank_game_mode_infinite_terrain_bp2))

(event `self.DestroyVolume.OnComponentBeginOverlap`
  (params (OverlappedComponent :type "PrimitiveComponent Object Reference") (OtherActor :type "Actor Object Reference") (OtherComp :type "PrimitiveComponent Object Reference") (OtherBodyIndex :type Integer) (bFromSweep :type Boolean) (SweepResult :type "HitResult Structure (by ref)"))
  (`self.IsPlayerActor` OtherActor)
  (`self.K2_DestroyActor`))

(fn `GetAttachLocation`
  (returns (`Attach Transform` :type "Transform Structure"))
  (return (`SceneComponent.K2_GetComponentToWorld` (`self.AttachPoint`))))

(fn `LockLevel`
  (`PrimitiveComponent.SetCollisionEnabled` (`self.Barrier`) "QueryAndPhysics")
  ;[1 1 1] Set Material - Unused at the moment
  (`PrimitiveComponent.SetMaterial` (`self.Barrier`) 0 "/Game/Static/Models/Mortar/glass.glass"))

(fn `UnlockLevel`
  (`PrimitiveComponent.SetCollisionEnabled` (`self.Barrier`) "NoCollision")
  ;[1 1 1] Set Barrier Material - Currently Unused
  (`PrimitiveComponent.SetMaterial` (`self.Barrier`) 0 "/Game/Static/Models/Mortar/blue.blue"))

(fn `UserConstructionScript`)