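; Sentry2_BP is a sentry unit built from tank parts: barrel, turret, tracks, and tank aiming and movement components.
; On BeginPlay it passes the barrel and turret to TankAiming and both tracks to TankMovement.
; It then casts its Widget component's user widget to HealthBar_BP and sets itself as that bar's Tank reference, linking the health display to this instance.
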(event `self.ReceiveBeginPlay`
  (`TankAimingComponent.InitializeAim` (`self.TankAiming`) (`self.TankBarrel`) (`self.TankTurret`))
  (`TankMovementComponent.Initialize` (`self.TankMovement`) (`self.LeftTrack`) (`self.RightTrack`))
  (`self.Initialize Health Widget`))

(fn `Initialize Health Widget`
  (bind _ashealth_bar_bp (cast `/Game/Dynamic/Blueprints/HealthBar_BP` (`WidgetComponent.GetUserWidgetObject` (`self.Widget`))))
  (set `/Game/Dynamic/Blueprints/HealthBar_BP.Tank` self _ashealth_bar_bp))

(fn `UserConstructionScript`)